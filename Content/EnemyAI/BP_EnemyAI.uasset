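; Enemy AI Blueprint that starts the BT_Chase behavior tree on BeginPlay, through the AI controller looked up from its owner.
; Its AIPerception update event only looks up the stimulus's sense class.
; The following sight logic is disconnected and never runs: it would set or clear the player as blackboard TargetActor and store LastKnownLocation on successful sensing.
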(event `self.ReceiveBeginPlay`
  (`AIController.RunBehaviorTree` (`AIBlueprintHelperLibrary.GetAIController` (`self.GetOwner`)) "/Game/EnemyAI/BT_Chase.BT_Chase"))

(event `self.AIPerception.OnTargetPerceptionUpdated`
  (params (Actor :type "Actor Object Reference") (Stimulus :type "AIStimulus Structure"))
  ;[1 1 1] If it sees player, it will check to see if it's the player. If it's the player, it will set the player as the value of the object. If it loses sight of the player, it will update the vector as the last known object.
  (bind _returnvalue (`AIPerceptionSystem.GetSenseClassForStimulus` Stimulus)))

(fn `UserConstructionScript`)